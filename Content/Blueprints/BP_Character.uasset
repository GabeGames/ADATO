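; BP_Character is a character Blueprint that manages the crosshair HUD and its interaction cue for computers.
; BeginPlay creates the WBP_Crosshair widget and adds it to the viewport, and the start and stop computer-use events remove and re-add it.
; Each Tick, a short Visibility line trace from the camera manager toggles the crosshair's interact state according to whether the hit actor casts to Computer.
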(event `self.ReceiveBeginPlay`
  (bind _returnvalue (`|CreateWidget` "/Game/UI/WBP_Crosshair.WBP_Crosshair_C" (`GameplayStatics.GetPlayerController` 0)))
  (bind _output_get (set `self.CrosshairWidget` _returnvalue))
  (`UserWidget.AddToViewport` _output_get 0))

(event `StartUsingComputer`
  (`Widget.RemoveFromParent` (`self.CrosshairWidget`)))

(event `StopUsingComputer`
  (`UserWidget.AddToViewport` (`self.CrosshairWidget`) 0))

(event `self.ReceiveTick`
  (params (DeltaSeconds :type "Float (single-precision)"))
  (bind _returnvalue (`GameplayStatics.GetPlayerCameraManager` 0))
  (bind _crosshairwidget (`self.CrosshairWidget`))
  (bind _returnvalue_2 (`self.K2_GetActorLocation` _returnvalue))
  (bind _outhit (`KismetSystemLibrary.LineTraceSingle` :`Start` _returnvalue_2 :`End` (+ _returnvalue_2 (* (`self.GetActorForwardVector` _returnvalue) 150.0)) :`TraceChannel` "TraceTypeQuery1" :`DrawTime` 0.0))
  (cast `/Game/Blueprints/Computer` (`.HitActor` (`GameplayStatics.BreakHitResult` _outhit))
    (:`then`
      (`/Game/UI/WBP_Crosshair.ToggleInteract` _crosshairwidget true))
    (:`CastFailed`
      (`/Game/UI/WBP_Crosshair.ToggleInteract` _crosshairwidget false))))

(fn `UserConstructionScript`)